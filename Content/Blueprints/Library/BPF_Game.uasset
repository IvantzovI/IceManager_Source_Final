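; Function library of shared helpers for an athlete team management game.
; Date helpers parse DD.MM.YYYY strings against the game instance's CurrentDate for age and past/present/future checks, the latter comparing day-of-year only.
; Competition helpers roll randomized scores from athlete stats, capped at 100, and test norms against team-type thresholds.
; Other helpers provide Russian display names, rich-text stat coloring, number formatting, a menu-map check and descending integer sort by repeated max extraction.
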(fn `CalculateCompetitionPointsByFormula`
  (params (Type :type "/Game/Data/E_CompetitionType Enum" :default "NewEnumerator0") (Athlete :type "/Game/Data/S_Athlete Structure"))
  (returns (Points :type Integer))
  (return (`KismetMathLibrary.FFloor` (`KismetMathLibrary.FMin` (select `/Game/Data/E_CompetitionType` (`local.Type`) :`NewEnumerator0` (+ (/ (+ Athlete_athlete_condition_90_E42C97F44D19DC73619237A5046044E2 Athlete_athlete_potential_91_372D3C5641EF8F81A7501B933FC6102D) 2.0) (`KismetMathLibrary.Conv_IntToDouble` (`KismetMathLibrary.RandomIntegerInRange` -10 30))) :`NewEnumerator1` (+ (/ (+ Athlete_athlete_condition_90_E42C97F44D19DC73619237A5046044E2 Athlete_athlete_potential_91_372D3C5641EF8F81A7501B933FC6102D) 4.0) (/ (* Athlete_athlete_potential_91_372D3C5641EF8F81A7501B933FC6102D (/ (+ Athlete_athlete_slip_92_B7DD2D24488D4007EFF1FE8ED2D473E7 Athlete_athlete_jumping_93_5FDE609E46157E8D18A4838452193CB7 Athlete_athlete_rotation_94_94DD7EFB4921FFE84272898C65F1A10B Athlete_athlete_dancing_95_A566E80A4630CCB50176E59C6ACFDB5C) 4.0)) 100.0) (`KismetMathLibrary.Conv_IntToDouble` (`KismetMathLibrary.RandomIntegerInRange` -10 30)))) 100.0))))

(fn `CalculateValueByFormula`
  (params (Params :type "/Game/Data/S_Formula Structure"))
  (returns (Value :type "Float (double-precision)"))
  (return (/ (`KismetMathLibrary.Conv_IntToDouble` (`KismetMathLibrary.RandomIntegerInRange` Params_RandMin_5_893F10B943467B1E59BBB782DDA143BE Params_RandMax_6_F164E40D4525F1F512EEF782AC25FA26)) (`KismetMathLibrary.Conv_IntToDouble` Params_Divider_8_169CD5674A9FFF37DC87868A98755768))))

(fn `CompareWithCurrentDate`
  (params (CompareDate :type String))
  (returns (Index :type "/Game/Data/E_CompetitionState Enum"))
  (bind _comparedate (`local.CompareDate`))
  (bind _returnvalue (`KismetMathLibrary.GetDayOfYear` (`KismetMathLibrary.MakeDateTime` (`KismetStringLibrary.Conv_StringToInt` (`KismetStringLibrary.GetSubstring` _comparedate 6 4)) (`KismetStringLibrary.Conv_StringToInt` (`KismetStringLibrary.GetSubstring` _comparedate 3 2)) (`KismetStringLibrary.Conv_StringToInt` (`KismetStringLibrary.GetSubstring` _comparedate 0 2)))))
  (bind _asbp_game_instance (cast `/Game/Blueprints/Game/BP_GameInstance` (`GameplayStatics.GetGameInstance` null)))
  (bind _returnvalue_2 (`KismetMathLibrary.GetDayOfYear` (`/Game/Blueprints/Game/BP_GameInstance.CurrentDate` _asbp_game_instance)))
  (return (select `bool` (< _returnvalue _returnvalue_2) :`false` (select `bool` (== _returnvalue _returnvalue_2) :`false` "NewEnumerator2" :`true` "NewEnumerator1" :!type "/Game/Data/E_CompetitionState Enum") :`true` "NewEnumerator0")))

(fn `GetAgeFromDate`
  (params (Date :type String))
  (returns (Age :type Integer))
  (bind _date (`local.Date`))
  (bind _asbp_game_instance (cast `/Game/Blueprints/Game/BP_GameInstance` (`GameplayStatics.GetGameInstance` null)))
  (return (/ (`KismetMathLibrary.GetDays` (- (`/Game/Blueprints/Game/BP_GameInstance.CurrentDate` _asbp_game_instance) (`KismetMathLibrary.MakeDateTime` (`KismetStringLibrary.Conv_StringToInt` (`KismetStringLibrary.GetSubstring` _date 6 4)) (`KismetStringLibrary.Conv_StringToInt` (`KismetStringLibrary.GetSubstring` _date 3 2)) (`KismetStringLibrary.Conv_StringToInt` (`KismetStringLibrary.GetSubstring` _date 0 2))))) 365)))

(fn `GetCompetitionNameByType`
  (params (Type :type "/Game/Data/E_CompetitionType Enum" :default "NewEnumerator0"))
  (returns (Name :type String))
  (return (select `/Game/Data/E_CompetitionType` Type :`NewEnumerator0` "Нормативы" :`NewEnumerator1` "Подводящие")))

(fn `GetMonthNameByIndex`
  (params (MonthIndex :type Integer))
  (returns (MonthName :type String))
  (return (select `int` (- MonthIndex 1) :`0` "Январь" :`1` "Февраль" :`2` "Март" :`3` "Апрель" :`4` "Май" :`5` "Июнь" :`6` "Июль" :`7` "Август" :`8` "Сентябрь" :`9` "Октябрь" :`10` "Ноябрь" :`11` "Декабрь")))

(fn `GetStatStateFromFloat`
  (params (Value :type "Float (double-precision)"))
  (returns (StatState :type "/Game/Data/E_StatState Enum"))
  (return (select `bool` (> Value 0.0) :`false` (select `bool` (== Value 0.0) :`false` "NewEnumerator2" :`true` "NewEnumerator0" :!type "/Game/Data/E_StatState Enum") :`true` "NewEnumerator1")))

(fn `GetStatTextFromState`
  (params (Text :type String) (State :type "/Game/Data/E_StatState Enum" :default "NewEnumerator0"))
  (returns (TextWithColor :type String))
  (return (select `/Game/Data/E_StatState` (`local.State`) :`NewEnumerator0` Text :`NewEnumerator1` (`KismetStringLibrary.Concat_StrStr` "<RichText.Green>" Text "</>") :`NewEnumerator2` (`KismetStringLibrary.Concat_StrStr` "<RichText.Red>" Text "</>"))))

(fn `GetTeamNameByIndex`
  (params (TeamIndex :type Integer))
  (returns (TeamName :type String))
  (return (select `int` TeamIndex :`0` "Первая" :`1` "Вторая" :`2` "Третья" :`3` "Четвертая" :`4` "Пятая")))

(fn `GetTeamTypeByIndex`
  (params (TeamIndex :type Integer))
  (returns (TeamName :type String))
  (return (select `int` TeamIndex :`0` "Детская" :`1` "Юношеская" :`2` "Юниорская" :`3` "Молодежная" :`4` "Взрослая")))

(fn `IsGameMap`
  (returns (bIsGameMap :type Boolean))
  (bind _returnvalue (`GameplayStatics.GetCurrentLevelName` null))
  (return (`KismetStringLibrary.NotEqual_StrStr` _returnvalue "M_Menu")))

(fn `IsNormsSuccessForAthlete`
  (params (TeamType :type "/Game/Data/E_TeamType Enum" :default "NewEnumerator0") (Points :type Integer))
  (returns (bSuccess :type Boolean))
  (return (>= Points (select `/Game/Data/E_TeamType` (`local.TeamType`) :`NewEnumerator0` 65 :`NewEnumerator1` 75))))

(fn `ReturnEmptyStringIfZero`
  (params (Value :type Integer))
  (returns (String :type String))
  (return (`KismetMathLibrary.SelectString` "" (`KismetStringLibrary.Conv_IntToString` (`local.Value`)) (== Value 0))))

(fn `ShortIntToString`
  (params (Int :type Integer))
  (returns (String :type String))
  (bind _returnvalue (`KismetStringLibrary.Conv_IntToString` Int))
  (return (`KismetMathLibrary.SelectString` (`KismetStringLibrary.Concat_StrStr` "0" _returnvalue) _returnvalue (< Int 10))))

(fn `SortIntegerArray`
  (params (InArray :type "Array of Integer"))
  (returns (OutArray :type "Array of Integer"))
  (locals (NewArray :type "Array of Integer") (TargetArray :type "Array of Integer"))
  (bind (_indexofmaxvalue _maxvalue) (`KismetMathLibrary.MaxOfIntArray` (`local.TargetArray`)))
  (set `local.TargetArray` InArray)
  (if (`KismetArrayLibrary.Array_IsValidIndex` (`local.TargetArray`)) :!label _label
    (`KismetArrayLibrary.Array_Add` (`local.NewArray`) _maxvalue)
    (`KismetArrayLibrary.Array_Remove` (`local.TargetArray`) _indexofmaxvalue)
    (goto _label)
    (else
      (return (`local.NewArray`)))))